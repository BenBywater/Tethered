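; Controller for the first UFO that also sets up and drives a second UFO from its own input bindings.
; On BeginPlay it spawns a UFO2Controller and a UFO2_BP pawn at one fixed spot, then has that controller possess the pawn.
; Both UFO2 axis events push the pawn along its control-rotation forward vector; the X event ignores its axis value and uses a constant scale.
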(event EventBeginPlay
  (bind _returnvalue (Math|Transform|MakeTransform "-50.000000,-300.000000,100.000000"))
  (bind _returnvalue_2 (Game|SpawnActorfromClass "/Game/Blueprints/UFO2Controller.UFO2Controller_C" _returnvalue "Undefined" 0 0))
  (bind _output_get (Variables|Default|SetUFO2Controller _returnvalue_2))
  (bind _returnvalue_3 (Game|SpawnActorfromClass "/Game/Blueprints/UFO2_BP.UFO2_BP_C" _returnvalue "Undefined" 0 0))
  (bind _output_get_2 (Variables|Default|SetUFO2Pawn _returnvalue_3))
  (Pawn|Possess _output_get _output_get_2))

(event EventTick
  (params (DeltaSeconds :type Float%20%28single-precision%29)))

(event Input|AxisEvents|InputAxisXAxisMovementUFO2
  (params (AxisValue :type Float%20%28single-precision%29))
  (bind _ufo2pawn (Variables|Default|GetUFO2Pawn))
  (Pawn|Input|AddMovementInput _ufo2pawn (Math|Vector|GetForwardVector (Pawn|GetControlRotation _ufo2pawn :!class /Script/Engine.Pawn)) 1.0 false))

(event Input|AxisEvents|InputAxisYAxisMovementUFO2
  (params (AxisValue :type Float%20%28single-precision%29))
  (bind _ufo2pawn (Variables|Default|GetUFO2Pawn))
  (Pawn|Input|AddMovementInput _ufo2pawn (Math|Vector|GetForwardVector (Pawn|GetControlRotation _ufo2pawn :!class /Script/Engine.Pawn)) AxisValue false))

(fn ConstructionScript)