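; Camera_BP is an actor that carries a Package component and two tether components linked to PlayerUFO actors.
; On BeginPlay it attaches each tether's end to one of the first two UFOs found.
; Every Tick, when the second UFO is over a distance threshold away, it moves the Package by a clamped step toward that UFO and prints the target.
; The world-space target is passed as a relative location.
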(event EventBeginPlay
  (bind _outactors (Actor|GetAllActorsOfClass "/Script/Tethered.PlayerUFO"))
  (Class|CableComponent|SetAttachEndto (Variables|Default|GetTetherUFO1) (Utilities|Array|Get(acopy) _outactors) "None" "TetherEnd")
  (Class|CableComponent|SetAttachEndto (Variables|Default|GetTetherUFO2) (Utilities|Array|Get(acopy) _outactors 1) "None" "TetherEnd"))

(event Collision|EventActorBeginOverlap
  (params (OtherActor :type Actor%20Object%20Reference)))

(event EventTick
  (params (DeltaSeconds :type Float%20%28single-precision%29))
  (bind _package (Variables|Default|GetPackage))
  (bind _outactors (Actor|GetAllActorsOfClass "/Script/Tethered.PlayerUFO"))
  (bind _output_get (Variables|Default|SetDistance (Transformation|GetDistanceTo (Utilities|Array|Get(acopy) _outactors 1) self)))
  (Math|Float|CompareFloat _output_get 1e+03
    (:>
      (bind _output_get_2 (Variables|Default|SetActorLocation (Transformation|GetActorLocation (Utilities|Array|Get(acopy) _outactors 1))))
      (bind _output_get_3 (Variables|Default|SetWorldLocation (Transformation|GetWorldLocation _package)))
      (Development|PrintString (Utilities|String|ToString(Vector) (+ (Math|Vector|ClampVectorSize (- _output_get_2 _output_get_3) -1e+01 1e+01) (Variables|Default|GetWorldLocation))))
      (Components|MoveComponentTo _package (+ (Math|Vector|ClampVectorSize (- _output_get_2 _output_get_3) -1e+01 1e+01) (Variables|Default|GetWorldLocation)) "0, 0, 0" false false 0.2 false))))

(fn ConstructionScript)